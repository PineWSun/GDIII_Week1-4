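; Base pressure plate that sinks while the player character (BP_Char2_JK1) stands on it and opens linked plant walls.
; Trigger overlap sets the character's IsInteracting flag and plays a timeline that lowers the plate; leaving clears the flag and reverses it.
; Every timeline update, in either direction, searches all Bp_plantwall1 actors and calls OpenGrass on those whose DoorValue matches PlateValue.
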(event `self.Trigger.OnComponentBeginOverlap`
  (params (OverlappedComponent :type "PrimitiveComponent Object Reference") (OtherActor :type "Actor Object Reference") (OtherComp :type "PrimitiveComponent Object Reference") (OtherBodyIndex :type Integer) (bFromSweep :type Boolean) (SweepResult :type "HitResult Structure (by ref)"))
  (bind _asbp_char_2_jk1 (cast `/Game/Developers/kraft/Blueprints/BP_Char2_JK1` OtherActor))
  (set `/Game/Developers/kraft/Blueprints/BP_Char2_JK1.isInteracting` true _asbp_char_2_jk1)
  (bind (_direction _plate_height) (`Timeline|PressurePlateTriggered` :!label _label)
    (:`Update`
      (`SceneComponent.K2_SetRelativeLocation` (`self.Plate`) (`KismetMathLibrary.MakeVector` 0.0 0.0 (`KismetMathLibrary.Lerp` 10.0 0.0 _plate_height)) false false)
      (bind _outactors (`GameplayStatics.GetAllActorsOfClass` "/Game/Drake_Dev_Folder/bp_plantwall1.bp_plantwall1_C"))
      (for _array_element _outactors
        (if (== (`/Game/Drake_Dev_Folder/bp_plantwall1.doorValue` _array_element) (`self.plateValue`))
          (`/Game/Drake_Dev_Folder/bp_plantwall1.OpenGrass` _array_element null))))))

(event `self.Trigger.OnComponentEndOverlap`
  (params (OverlappedComponent :type "PrimitiveComponent Object Reference") (OtherActor :type "Actor Object Reference") (OtherComp :type "PrimitiveComponent Object Reference") (OtherBodyIndex :type Integer))
  (bind _asbp_char_2_jk1 (cast `/Game/Developers/kraft/Blueprints/BP_Char2_JK1` OtherActor))
  (set `/Game/Developers/kraft/Blueprints/BP_Char2_JK1.isInteracting` false _asbp_char_2_jk1)
  (goto _label :!via `Reverse`))

(fn `UserConstructionScript`)