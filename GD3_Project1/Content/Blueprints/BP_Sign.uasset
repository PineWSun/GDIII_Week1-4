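; BP_Sign is an interactable sign that opens matching plant walls.
; It creates a P_interact prompt on BeginPlay and shows or hides it as the player pawn enters or leaves its Box.
; On Interact it plays a click, then searches all Bp_plantwall1 actors and calls OpenGrass on those whose DoorValue equals its ButtonValue, with a leaves sound.
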(event `self.ReceiveBeginPlay`
  (bind _returnvalue (`|GenericCreateObject` "/Game/Developers/kraft/Blueprints/p_interact.p_interact_C"))
  (set `self.interactPrompt` _returnvalue))

(event `self.Box.OnComponentBeginOverlap`
  (params (OverlappedComponent :type "PrimitiveComponent Object Reference") (OtherActor :type "Actor Object Reference") (OtherComp :type "PrimitiveComponent Object Reference") (OtherBodyIndex :type Integer) (bFromSweep :type Boolean) (SweepResult :type "HitResult Structure (by ref)"))
  (if (== OtherActor (`GameplayStatics.GetPlayerPawn` 0))
    (`UserWidget.AddToViewport` (`self.interactPrompt`) 0)))

(event `self.Box.OnComponentEndOverlap`
  (params (OverlappedComponent :type "PrimitiveComponent Object Reference") (OtherActor :type "Actor Object Reference") (OtherComp :type "PrimitiveComponent Object Reference") (OtherBodyIndex :type Integer))
  (if (== (`GameplayStatics.GetPlayerPawn` 0) OtherActor)
    (`Widget.RemoveFromParent` (`self.interactPrompt`))))

(event `/Game/Developers/kraft/Blueprints/InteractInterface.Interact`
  (params (Player :type "Actor Object Reference"))
  (`GameplayStatics.PlaySound2D` "/Game/Blueprints/clicksfx.clicksfx" 1.0 1.0 0.0 null null)
  (bind _outactors (`GameplayStatics.GetAllActorsOfClass` "/Game/Drake_Dev_Folder/bp_plantwall1.bp_plantwall1_C"))
  (for _array_element _outactors
    (if (== (`/Game/Drake_Dev_Folder/bp_plantwall1.doorValue` _array_element) (`self.buttonValue`))
      (`/Game/Drake_Dev_Folder/bp_plantwall1.OpenGrass` _array_element Player)
      (`GameplayStatics.PlaySound2D` "/Game/Blueprints/leavessfx.leavessfx" 1.0 1.0 0.0 null null))))

(fn `UserConstructionScript`)