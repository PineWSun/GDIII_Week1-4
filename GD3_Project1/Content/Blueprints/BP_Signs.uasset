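; BP_Signs is a sign actor that displays editable text through several text render components.
; Its construction script copies the TextSign, Sign2, Sign3, Sign4 and Sign6 variables into five text renders, with no assignment for TextRender4.
; The event graph holds only empty, disabled default events, so the Blueprint adds no gameplay logic.
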(fn `UserConstructionScript`
  (`TextRenderComponent.K2_SetText` (`self.TextRender`) (`self.TextSign`))
  (`TextRenderComponent.K2_SetText` (`self.TextRender1`) (`self.Sign2`))
  (`TextRenderComponent.K2_SetText` (`self.TextRender2`) (`self.Sign3`))
  (`TextRenderComponent.K2_SetText` (`self.TextRender3`) (`self.Sign4`))
  (`TextRenderComponent.K2_SetText` (`self.TextRender5`) (`self.Sign6`)))